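; Local multiplayer manager that handles menu screens, level changes and the timed elimination round.
; It spawns and possesses an InputReciver per tagged PlayerStart, carrying active player indices between levels through mainInstance.
; Each round, the DeathPick timeline runs until all but one living player jumps or time expires, then tags a random non-jumper.
; The Levelloop timeline feeds the PIXY-ItsTime countdown widget and kills whoever is tagged when it finishes.
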(event `start game`
  (`KismetArrayLibrary.Array_Clear` (`self.AlivePlayersArray`))
  (bind _outactors (`GameplayStatics.GetAllActorsOfClass` "/Game/Gio/BP_Player.BP_Player_C"))
  (for _array_element _outactors
    (if (`/Game/Gio/BP_Player.Alive` _array_element)
      (`KismetArrayLibrary.Array_Add` (`self.AlivePlayersArray`) _array_element)))
  (`self.Pick Death setup`)
  (`Timeline|DeathPick` :`NewTime` 0.0 :!label _label
    (:`Update`
      (set `self.jumped` 0)
      (for _array_element_2 (`self.AlivePlayersArray`)
        (if (`/Game/Gio/BP_Player.jumped` _array_element_2)
          (`/Engine/EditorBlueprintResources/StandardMacros.IncrementInt` (`self.jumped`))))
      (if (>= (`self.jumped`) (- (`KismetArrayLibrary.Array_Length` (`self.AlivePlayersArray`)) 1))
        (`|ExecutionSequence`
          (:`then_0`
            (goto _label :!via `Stop`))
          (:`then_1`
            (`KismetArrayLibrary.Array_Clear` (`self.Antijumped players array`) :!label _label_2)
            (for _array_element_3 (`self.AlivePlayersArray`)
              (set `/Game/Gio/BP_Player.IT TICKLE TIME OH NO` false _array_element_3)
              (if (not (`/Game/Gio/BP_Player.jumped` _array_element_3))
                (`KismetArrayLibrary.Array_Add` (`self.Antijumped players array`) _array_element_3)))
            (set `/Game/Gio/BP_Player.IT TICKLE TIME OH NO` true (`KismetArrayLibrary.Array_Random` (`self.Antijumped players array`)))
            (bind _aspixy_its_time (cast `/Game/Bob/PIXY-ItsTime` (`self.widgets`)))
            (`/Game/Bob/PIXY-ItsTime.set jump visability` _aspixy_its_time false)
            (bind (_direction _newtrack_0) (`Timeline|levelloop` :!label _label_3)
              (:`Update`
                (set `self.time left` _newtrack_0)
                (bind _aspixy_its_time_2 (cast `/Game/Bob/PIXY-ItsTime` (`self.widgets`)))
                (set `/Game/Bob/PIXY-ItsTime.time lesft` (`self.time left`) _aspixy_its_time_2))
              (:`Finished`
                (for _array_element_4 (`self.AlivePlayersArray`)
                  (if (`/Game/Gio/BP_Player.IT TICKLE TIME OH NO` _array_element_4)
                    (`/Game/Gio/BP_Player.Death` _array_element_4)))))))))
    (:`Finished`
      (goto _label_2))))

(event `end game`
  (goto _label_3 :!via `Stop`))

(event `self.ReceiveBeginPlay`
  (bind _asmain_instance (cast `/Game/Gio/mainInstance` (`GameplayStatics.GetGameInstance`)))
  (if (`/Game/Gio/mainInstance.menu` _asmain_instance)
    (bind _returnvalue (`|CreateWidget` "/Game/Gio/widets/WBP_MainMenu.WBP_MainMenu_C"))
    (set `self.widgets` _returnvalue)
    (`UserWidget.AddToViewport` _returnvalue 0)
    (set `PlayerController.bShowMouseCursor` true (`GameplayStatics.GetPlayerController` 0)))
  (`self.GetPlayerStartPoints`)
  (`self.SpawnInputRecivers`)
  (bind _outactors (`GameplayStatics.GetAllActorsOfClass` "/Game/Gio/Display_Charector.Display_Charector_C"))
  (bind _output_get (set `self.DisplayCharectorArray` _outactors))
  (for _array_element _output_get
    (set `/Game/Gio/Display_Charector.inputreciver` (`|GetArrayItem` (`self.InputReciverArray`) (`/Game/Gio/Display_Charector.index` _array_element)) _array_element)))

(fn `call start game`
  (`self.start game`))

(fn `CreateFirstPlayer`
  (for _array_element (`self.InputReciverArray`)
    (if (== (`/Game/Gio/InputReciver.PlayerIndex` _array_element) 0)
      (set `/Game/Gio/InputReciver.active` true _array_element))))

(fn `credits`
  (returns (`return 0` :type Boolean))
  (`Widget.RemoveFromParent` (`self.widgets`))
  (bind _asmain_instance (cast `/Game/Gio/mainInstance` (`GameplayStatics.GetGameInstance`)))
  (set `/Game/Gio/mainInstance.menu` false _asmain_instance)
  (`GameplayStatics.OpenLevelBySoftObjectPtr` "/Game/Bob/Credits.Credits")
  (return false))

(fn `GetPlayerStartPoints`
  (bind _outactors (`GameplayStatics.GetAllActorsOfClass` "/Script/Engine.PlayerStart"))
  (set `self.PlayerStartArray` _outactors))

(fn `howToPlay`
  (returns (`return 0` :type Boolean))
  (`Widget.RemoveFromParent` (`self.widgets`))
  (bind _returnvalue (`|CreateWidget` "/Game/Gio/widets/WBP_htp.WBP_htp_C"))
  (set `self.widgets` _returnvalue)
  (`UserWidget.AddToViewport` _returnvalue 0)
  (return false))

(fn `LoadLevel`
  (params (LevelName :type Name))
  (returns (return0 :type Boolean))
  (set `PlayerController.bShowMouseCursor` false (`GameplayStatics.GetPlayerController` 0))
  (`self.ResetArrays`)
  (`GameplayStatics.OpenLevel` LevelName)
  (return false))

(fn `main menu`
  (returns (`return 0` :type Boolean))
  (`Widget.RemoveFromParent` (`self.widgets`))
  (bind _returnvalue (`|CreateWidget` "/Game/Gio/widets/WBP_MainMenu.WBP_MainMenu_C"))
  (set `self.widgets` _returnvalue)
  (`UserWidget.AddToViewport` _returnvalue 0)
  (return false))

(fn `Pick Death setup`
  (for _array_element (`self.AlivePlayersArray`)
    (set `/Game/Gio/BP_Player.jumped` false _array_element))
  (bind _aspixy_its_time (cast `/Game/Bob/PIXY-ItsTime` (`self.widgets`)))
  (`/Game/Bob/PIXY-ItsTime.set jump visability` _aspixy_its_time true))

(fn `ResetArrays`
  (for _array_element (`self.PlayerControllerArray`)
    (`GameplayStatics.RemovePlayer` _array_element))
  (`KismetArrayLibrary.Array_Clear` (`self.PlayerStartArray`))
  (for _array_element_2 (`self.InputReciverArray`)
    (if (`/Game/Gio/InputReciver.active` _array_element_2)
      (`KismetArrayLibrary.Array_AddUnique` (`self.ActivePlayersIndex`) (`/Game/Gio/InputReciver.PlayerIndex` _array_element_2))))
  (`KismetArrayLibrary.Array_Clear` (`self.InputReciverArray`))
  (`Widget.RemoveFromParent` (`self.widgets`))
  (bind _asmain_instance (cast `/Game/Gio/mainInstance` (`GameplayStatics.GetGameInstance`)))
  (set `/Game/Gio/mainInstance.activeIndex` (`self.ActivePlayersIndex`) _asmain_instance)
  (set `/Game/Gio/mainInstance.menu` false _asmain_instance))

(fn `Settings`
  (returns (`return 0` :type Boolean))
  (`Widget.RemoveFromParent` (`self.widgets`))
  (bind _returnvalue (`|CreateWidget` "/Game/Gio/widets/WBP_settings.WBP_settings_C"))
  (set `self.widgets` _returnvalue)
  (`UserWidget.AddToViewport` _returnvalue 0)
  (return false))

(fn `SpawnInputRecivers`
  (locals (index :type Integer))
  (bind _index (`local.index`))
  (bind _returnvalue (`GameplayStatics.GetPlayerController` (`local.index`)))
  (for (_ _array_index) (`self.PlayerStartArray`)
    (set `local.index` _array_index)
    (for _array_element (`self.PlayerStartArray`)
      (if (== (`local.index`) (`KismetStringLibrary.Conv_StringToInt` (`KismetStringLibrary.Conv_NameToString` (`PlayerStart.PlayerStartTag` _array_element))))
        (`GameplayStatics.CreatePlayer` -1)
        (bind _returnvalue_2 (`|SpawnActorFromClass` "/Game/Gio/InputReciver.InputReciver_C" (`self.GetTransform` (`|GetArrayItem` (`self.PlayerStartArray`) _index)) "Undefined" "OverrideRootScale" null _index null))
        (set `/Game/Gio/InputReciver.active` (`KismetArrayLibrary.Array_Contains` (`self.ActivePlayersIndex`) (`local.index`)) _returnvalue_2)
        (`KismetArrayLibrary.Array_AddUnique` (`self.InputReciverArray`) _returnvalue_2)
        (`Controller.Possess` _returnvalue _returnvalue_2)
        (`KismetArrayLibrary.Array_AddUnique` (`self.PlayerControllerArray`) _returnvalue)))))

(fn `SpwanPlayer`
  (params (CurrentPlayerIndex :type Integer) (InputReciver :type "/Game/Gio/InputReciver Object Reference"))
  (returns (`Return 0` :type Boolean))
  (bind _returnvalue (`GameplayStatics.GetPlayerController` (`local.CurrentPlayerIndex`)))
  (bind _returnvalue_2 (`|SpawnActorFromClass` "/Game/Gio/BP_Player.BP_Player_C" (`self.GetTransform` InputReciver) "Undefined" "OverrideRootScale" null CurrentPlayerIndex null))
  (`Controller.Possess` _returnvalue _returnvalue_2)
  (bind _outactors (`GameplayStatics.GetAllActorsOfClass` "/Game/Bob/ComradeCam.ComradeCam_C"))
  (`PlayerController.SetViewTargetWithBlend` _returnvalue (`|GetArrayItem` _outactors) 0.0 "VTBlend_Linear" 0.0 false)
  (return false))

(fn `StartLevel`
  (returns (`Return 0` :type Boolean))
  (bind _asmain_instance (cast `/Game/Gio/mainInstance` (`GameplayStatics.GetGameInstance`)))
  (set `self.ActivePlayersIndex` (`/Game/Gio/mainInstance.activeIndex` _asmain_instance))
  (`self.GetPlayerStartPoints`)
  (`self.SpawnInputRecivers`)
  (for _array_element (`self.InputReciverArray`)
    (`/Game/Gio/InputReciver.StartLevel` _array_element))
  (`KismetArrayLibrary.Array_Clear` (`self.ActivePlayersIndex`))
  (`self.time and pointer`)
  (`self.call start game`)
  (return false))

(fn `time and pointer`
  (returns (`return 0` :type Boolean))
  (bind _returnvalue (`|CreateWidget` "/Game/Bob/PIXY-ItsTime.PIXY-ItsTime_C"))
  (set `self.widgets` _returnvalue)
  (`UserWidget.AddToViewport` _returnvalue 0)
  (return false))

(fn `UserConstructionScript`)