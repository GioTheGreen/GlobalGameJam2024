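; Base pickup item Blueprint that highlights under the mouse cursor and destroys itself when clicked.
; On BeginPlay it enables input and mouse-over events on the first player controller.
; Cursor enter and exit swap the first material slot of ItemModel between highlighted and standard materials, with the standard one also applied in the construction script.
; Hover and click events also print debug strings; clicking grants nothing here.
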(event `self.ReceiveBeginPlay`
  (bind _returnvalue (`GameplayStatics.GetPlayerController` 0))
  (`self.EnableInput` _returnvalue)
  (set `PlayerController.bEnableMouseOverEvents` true _returnvalue))

(event `self.ReceiveActorBeginCursorOver`
  (`KismetSystemLibrary.PrintString` "Hello")
  (`PrimitiveComponent.SetMaterial` (`self.Item_Model`) 0 (`self.Highlighted_Material`)))

(event `self.ReceiveActorEndCursorOver`
  (`KismetSystemLibrary.PrintString` "goodbye")
  (`PrimitiveComponent.SetMaterial` (`self.Item_Model`) 0 (`self.Standard_Material`)))

(event `self.ReceiveActorOnClicked`
  (params (ButtonPressed :type "Key Structure"))
  (`KismetSystemLibrary.PrintString` "Hello")
  (`self.K2_DestroyActor`))

(fn `UserConstructionScript`
  (`parent.UserConstructionScript`)
  (`PrimitiveComponent.SetMaterial` (`self.Item_Model`) 0 (`self.Standard_Material`)))