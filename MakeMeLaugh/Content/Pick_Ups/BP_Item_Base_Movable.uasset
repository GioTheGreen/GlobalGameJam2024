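; Base movable pickup item that repeatedly slides along its local X axis and snaps back to where it started.
; BeginPlay stores the start location, runs MoveX on a looping timer for stepped local offsets, and uses a looping Delay to reset the position every few seconds.
; Beginning an overlap only prints a debug message, while ending one destroys the actor.
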(event `self.ReceiveBeginPlay`
  (set `self.Original_Vector3` (`self.K2_GetActorLocation`))
  (`KismetSystemLibrary.K2_SetTimer` null "MoveX" 0.1 true :!label _label)
  (`KismetSystemLibrary.Delay` 3.0)
  (`self.K2_SetActorLocation` (`self.Original_Vector3`))
  (goto _label))

(event `self.ReceiveActorBeginOverlap`
  (params (OtherActor :type "Actor Object Reference"))
  (`KismetSystemLibrary.PrintString` "overlap began "))

(event `self.ReceiveActorEndOverlap`
  (params (OtherActor :type "Actor Object Reference"))
  (`self.K2_DestroyActor`))

(fn `MoveX`
  (`self.K2_AddActorLocalOffset` (10.0 0.0 0.0)))

(fn `UserConstructionScript`
  (`parent.UserConstructionScript`))